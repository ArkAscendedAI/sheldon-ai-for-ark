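; BP_SheldonDinoEventBuff is a dino buff that reports the death of its instigator dino over a WebSocket.
; On death, it builds a "dino_death" JSON string by concatenation from the dino's descriptive name, targeting team and damage causer's object name.
; It sends that string through the BP_SheldonWebSocket component on every BP_SheldonMapExtension actor.
; The damage adjustment override only passes through to the parent.
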(event `self.BPInstigatorDied`
  (params (DamageCauser :type "Actor Object Reference"))
  (bind _asprimal_dino_character (cast `PrimalDinoCharacter` (`self.Instigator`)))
  (bind _outactors (`GameplayStatics.GetAllActorsOfClass` null "/SheldonAI/Blueprints/BP_SheldonMapExtension.BP_SheldonMapExtension_C"))
  (for _array_element _outactors
    (`/SheldonAI/Blueprints/BP_SheldonWebSocket.SendPlayerMessage` (`self.GetComponentByClass` _array_element "/SheldonAI/Blueprints/BP_SheldonWebSocket.BP_SheldonWebSocket_C") (`KismetStringLibrary.Concat_StrStr` (`KismetStringLibrary.Concat_StrStr` (`KismetStringLibrary.Concat_StrStr` (`KismetStringLibrary.Concat_StrStr` (`KismetStringLibrary.Concat_StrStr` (`KismetStringLibrary.Concat_StrStr` "{\"type\":\"dino_death\",\"dino\":\"" (`PrimalDinoCharacter.GetDescriptiveName` _asprimal_dino_character)) "\",\"team\":") (`KismetStringLibrary.Conv_IntToString` (`PrimalDinoCharacter.TargetingTeam` _asprimal_dino_character))) ",\"killer\":\"") (`KismetSystemLibrary.GetObjectName` DamageCauser)) "\"}"))))

(fn `BPAdjustDamage_Ex`
  (params (Damage :type "Float (single-precision)") (HitInfo :type "HitResult Structure (by ref)") (ImpulseDir :type "Vector Structure (by ref)") (EventInstigator :type "Controller Object Reference") (InDamageCauser :type "Actor Object Reference") (TheDamgeType :type "DamageType Class Reference"))
  (returns (ReturnValue :type "Float (single-precision)"))
  (bind _returnvalue (`parent.BPAdjustDamage_Ex` Damage HitInfo ImpulseDir EventInstigator InDamageCauser TheDamgeType))
  (return _returnvalue))

(fn `UserConstructionScript`)