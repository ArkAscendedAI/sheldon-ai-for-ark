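; WebSocket client Blueprint that links a player to an external SheldonAI bridge for sending messages.
; ConnectToBridge reads URL and secret from ShooterGameMode options and opens the socket; SendAuthMessage sends hand-built JSON with player identity and placeholder position.
; Custom events handle open, failure with delayed retry, close, and substring-matched responses, which are only printed; player messages require authentication.
; BeginPlay is empty, and no event binding appears; the auth payload, secret included, is debug-printed.
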(event `CustomEvent`
  (set `self.IsConnected` true)
  (`self.SendAuthMessage`))

(event `CustomEvent_1`
  (set `self.IsConnected` false)
  (`KismetSystemLibrary.PrintString` null "Connection failed, retrying in 5s...")
  (`KismetSystemLibrary.Delay` null 5.0)
  (`self.ConnectToBridge`))

(event `CustomEvent_2`
  (set `self.IsConnected` false)
  (set `self.IsAuthenticated` false)
  (`KismetSystemLibrary.PrintString` null "WebSocket closed"))

(event `CustomEvent_3`
  (params (Message :type String))
  (`KismetSystemLibrary.PrintString` null Message)
  (if (`KismetStringLibrary.Contains` Message "auth_success")
    (set `self.IsAuthenticated` true)
    (`KismetSystemLibrary.PrintString` null "Authenticated!")
    (elif (`KismetStringLibrary.Contains` Message "\\\"type\\\":\\\"reply\\\"")
      (`KismetSystemLibrary.PrintString` null Message)
      (elif (`KismetStringLibrary.Contains` Message "\\\"type\\\":\\\"error\\\"")
        (`KismetSystemLibrary.PrintString` null "Error from bridge")))))

(fn `ConnectToBridge`
  (`self.ReadConfig`)
  (bind _returnvalue (`VictoryCore.CreateWebSocket` (`self.BridgeURL`)))
  (set `self.SocketID` _returnvalue)
  (if (>= (`self.SocketID`) 0)
    (`VictoryCore.WebSocketConnect` (`self.SocketID`))
    (else
      (`KismetSystemLibrary.PrintString` null "WebSocket creation failed"))))

(fn `Disconnect`
  (if (`self.IsConnected`)
    (`VictoryCore.WebSocketClose` (`self.SocketID`))
    (set `self.IsConnected` false)
    (set `self.IsAuthenticated` false)
    (set `self.SocketID` -1)))

(fn `ReadConfig`
  (bind _asshooter_game_mode (cast `ShooterGameMode` (`GameplayStatics.GetGameMode` null)))
  (bind _returnvalue (`ShooterGameMode.GetStringOption` _asshooter_game_mode "SheldonAI" "WebSocketURL"))
  (set `self.BridgeURL` _returnvalue)
  (bind _returnvalue_2 (`ShooterGameMode.GetStringOption` _asshooter_game_mode "SheldonAI" "AuthSecret"))
  (set `self.AuthSecret` _returnvalue_2))

(fn `SendAuthMessage`
  (bind _returnvalue (`KismetStringLibrary.Concat_StrStr` (`KismetStringLibrary.Concat_StrStr` (`KismetStringLibrary.Concat_StrStr` (`KismetStringLibrary.Concat_StrStr` (`KismetStringLibrary.Concat_StrStr` (`KismetStringLibrary.Concat_StrStr` (`KismetStringLibrary.Concat_StrStr` (`KismetStringLibrary.Concat_StrStr` "{\"type\":\"auth\",\"token\":\"" (`self.AuthSecret`)) "\",\"player\":{\"player_id\":\"") (`self.PlayerID`)) "\",\"display_name\":\"") (`self.PlayerName`)) "\",\"tier\":\"") (`self.PlayerTier`)) "\",\"tribe_id\":\"\",\"position\":{\"x\":0,\"y\":0,\"z\":0},\"facing_yaw\":0.0}}"))
  (`VictoryCore.WebSocketSendMessage` (`self.SocketID`) _returnvalue)
  (`KismetSystemLibrary.PrintString` null _returnvalue))

(fn `SendPlayerMessage`
  (params (Message :type String))
  (if (`self.IsAuthenticated`)
    (`VictoryCore.WebSocketSendMessage` (`self.SocketID`) (`KismetStringLibrary.Concat_StrStr` (`KismetStringLibrary.Concat_StrStr` "{\"type\":\"player_message\",\"message\":\"" Message) "\",\"position\":{\"x\":0,\"y\":0,\"z\":0},\"facing_yaw\":0.0}"))
    (else
      (`KismetSystemLibrary.PrintString` null "Not connected"))))