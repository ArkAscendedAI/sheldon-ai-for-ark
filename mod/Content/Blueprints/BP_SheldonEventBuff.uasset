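; Event-reporting buff that relays its owner's deaths, dino tames and damage taken to the Sheldon WebSocket.
; Each hook builds a JSON string by concatenation and sends it through the BP_SheldonWebSocket component on every BP_SheldonMapExtension actor.
; Damage reports require a player state, are throttled to a few seconds apart and return the incoming damage unchanged.
; Taming also calls StaticAddBuff on the new dino.
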(event `self.BPInstigatorDied`
  (params (DamageCauser :type "Actor Object Reference"))
  (bind _returnvalue (`Pawn.GetController` (`self.Instigator`)))
  (bind _asshooter_player_controller (cast `ShooterPlayerController` _returnvalue)
    (:`then`
      (bind _asshooter_player_state (cast `ShooterPlayerState` (`Controller.PlayerState` _returnvalue))
        (:`then`
          (bind _returnvalue_2 (`ShooterPlayerState.GetUniqueNetIdAsString` _asshooter_player_state)))
        (:`CastFailed`
          _)))
    (:`CastFailed`
      _))
  (bind _outactors (`GameplayStatics.GetAllActorsOfClass` null "/SheldonAI/Blueprints/BP_SheldonMapExtension.BP_SheldonMapExtension_C"))
  (for _array_element _outactors
    (`/SheldonAI/Blueprints/BP_SheldonWebSocket.SendPlayerMessage` (`self.GetComponentByClass` _array_element "/SheldonAI/Blueprints/BP_SheldonWebSocket.BP_SheldonWebSocket_C") (`KismetStringLibrary.Concat_StrStr` (`KismetStringLibrary.Concat_StrStr` (`KismetStringLibrary.Concat_StrStr` (`KismetStringLibrary.Concat_StrStr` "{\"type\":\"death\",\"killer\":\"" (`KismetSystemLibrary.GetObjectName` DamageCauser)) "\",\"victim\":\"") _returnvalue_2) "\"}"))))

(event `self.BPOnTamedWildDino`
  (params (Dino :type "PrimalDinoCharacter Object Reference"))
  (`parent.BPOnTamedWildDino` Dino)
  (bind _outactors (`GameplayStatics.GetAllActorsOfClass` null "/SheldonAI/Blueprints/BP_SheldonMapExtension.BP_SheldonMapExtension_C"))
  (for _array_element _outactors
    (`/SheldonAI/Blueprints/BP_SheldonWebSocket.SendPlayerMessage` (`self.GetComponentByClass` _array_element "/SheldonAI/Blueprints/BP_SheldonWebSocket.BP_SheldonWebSocket_C") (`KismetStringLibrary.Concat_StrStr` (`KismetStringLibrary.Concat_StrStr` (`KismetStringLibrary.Concat_StrStr` (`KismetStringLibrary.Concat_StrStr` (`KismetStringLibrary.Concat_StrStr` (`KismetStringLibrary.Concat_StrStr` "{\"type\":\"dino_tamed\",\"dino\":\"" (`PrimalDinoCharacter.GetDescriptiveName` Dino)) "\",\"team\":") (`KismetStringLibrary.Conv_IntToString` (`PrimalDinoCharacter.TargetingTeam` Dino))) ",\"tribe\":\"") (`PrimalDinoCharacter.TribeName` Dino)) "\"}")))
  (`self.StaticAddBuff` null Dino null null))

(fn `BPAdjustDamage_Ex`
  (params (Damage :type "Float (single-precision)") (HitInfo :type "HitResult Structure (by ref)") (ImpulseDir :type "Vector Structure (by ref)") (EventInstigator :type "Controller Object Reference") (InDamageCauser :type "Actor Object Reference") (TheDamgeType :type "DamageType Class Reference"))
  (returns (ReturnValue :type "Float (single-precision)"))
  (bind _returnvalue (`KismetSystemLibrary.GetGameTimeInSeconds` null))
  (`parent.BPAdjustDamage_Ex` Damage HitInfo ImpulseDir EventInstigator InDamageCauser TheDamgeType)
  (if (>= (- _returnvalue (`self.LastDamageSentTime`)) 3.0)
    (bind _asshooter_player_state (cast `ShooterPlayerState` (`Controller.PlayerState` (`Pawn.GetController` (`self.Instigator`))))
      (:`then`
        (bind _returnvalue_2 (`ShooterPlayerState.GetUniqueNetIdAsString` _asshooter_player_state))
        (bind _outactors (`GameplayStatics.GetAllActorsOfClass` null "/SheldonAI/Blueprints/BP_SheldonMapExtension.BP_SheldonMapExtension_C"))
        (for _array_element _outactors
          (`/SheldonAI/Blueprints/BP_SheldonWebSocket.SendPlayerMessage` (`self.GetComponentByClass` _array_element "/SheldonAI/Blueprints/BP_SheldonWebSocket.BP_SheldonWebSocket_C") (`KismetStringLibrary.Concat_StrStr` (`KismetStringLibrary.Concat_StrStr` (`KismetStringLibrary.Concat_StrStr` (`KismetStringLibrary.Concat_StrStr` (`KismetStringLibrary.Concat_StrStr` (`KismetStringLibrary.Concat_StrStr` "{\"type\":\"damage_event\",\"victim\":\"" _returnvalue_2) "\",\"amount\":") (`KismetStringLibrary.Conv_DoubleToString` Damage)) ",\"cause\":\"") (`KismetSystemLibrary.GetObjectName` InDamageCauser)) "\"}"))))
      (:`CastFailed`
        _))
    (set `self.LastDamageSentTime` _returnvalue))
  (return Damage))

(fn `UserConstructionScript`)