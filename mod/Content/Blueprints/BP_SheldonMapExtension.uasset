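; ARK map extension for Sheldon, an in-game chat assistant with an F8 chat window and subtitle replies.
; Server net exec forwards player ID, admin flag, name and message through SheldonWebSocket; its ConnectToBridge call is unwired here.
; Replies arrive via client net exec or RepNotify strings filtered by player ID, which also drive minimap pins and console commands.
; A looping timer applies BP_SheldonInputBuff to all ShooterCharacters.
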(event `self.ReceiveBeginPlay`
  (`parent.ReceiveBeginPlay`)
  (`/Engine/EditorBlueprintResources/ActorMacros.Switch Has Authority`
    (:`Authority`
      _)
    (:`Remote`
      _))
  (`self.EnableInput` (`GameplayStatics.GetPlayerController` null))
  (bind _returnvalue (`|CreateWidget` "/SheldonAI/Widgets/WBP_SheldonChat.WBP_SheldonChat_C"))
  (set `/SheldonAI/Widgets/WBP_SheldonChat.MapExtensionRef` self _returnvalue)
  (set `self.ChatWidget` _returnvalue)
  (`KismetSystemLibrary.K2_SetTimer` null "SweepPlayerBuffs" 10.0 true))

(event `Key|F8`
  (params (Key :type "Key Structure"))
  (bind _returnvalue (`GameplayStatics.GetPlayerController` null))
  (:`Pressed`
    (if (`self.IsWidgetOpen`)
      (`PrimalUserWidget.RemoveFromViewport` (`self.ChatWidget`))
      (`WidgetBlueprintLibrary.SetInputMode_GameOnly` null)
      (bind _asprimal_player_controller (cast `PrimalPlayerController` (`GameplayStatics.GetPlayerController` null)))
      (set `PrimalPlayerController.bForceShowMouseCursor` false _asprimal_player_controller)
      (set `self.IsWidgetOpen` false)
      (else
        (`PrimalUserWidget.AddToViewport` (`self.ChatWidget`) 0)
        (`WidgetBlueprintLibrary.SetInputMode_UIOnlyEx` _returnvalue (`/SheldonAI/Widgets/WBP_SheldonChat.MessageInput` (`self.ChatWidget`)))
        (bind _asprimal_player_controller_2 (cast `PrimalPlayerController` _returnvalue))
        (set `PrimalPlayerController.bForceShowMouseCursor` true _asprimal_player_controller_2)
        (set `self.IsWidgetOpen` true)
        (`KismetSystemLibrary.Delay` null 0.1)
        (`ScrollBox.ScrollToEnd` (`/SheldonAI/Widgets/WBP_SheldonChat.ChatScrollBox` (`self.ChatWidget`)))))))

(fn `BPClientHandleNetExecCommand`
  (params (CommandName :type Name) (ExecParams :type "BPNetExecParams Structure (by ref)") (ForPC :type "PlayerController Object Reference"))
  (returns (ReturnValue :type Boolean))
  (bind ((`StringParam1` _stringparam1)) (break `BPNetExecParams` ExecParams))
  (bind _chatwidget (`self.ChatWidget`))
  (bind _subtitlewidget (`self.SubtitleWidget`))
  (if (== CommandName "SheldonReply")
    (set `/SheldonAI/Widgets/WBP_SheldonChat.SheldonMsg` _stringparam1 _chatwidget)
    (`/SheldonAI/Widgets/WBP_SheldonChat.SheldonRenderMessage` _chatwidget)
    (if (not (`KismetSystemLibrary.IsValid` _subtitlewidget))
      (bind _returnvalue (`|CreateWidget` "/SheldonAI/Widgets/WBP_SheldonSubtitle.WBP_SheldonSubtitle_C" ForPC))
      (set `self.SubtitleWidget` _returnvalue)
      (`PrimalUserWidget.AddToViewport` _subtitlewidget 100))
    (`/SheldonAI/Widgets/WBP_SheldonSubtitle.ShowSubtitle` _subtitlewidget (`KismetTextLibrary.Conv_StringToText` _stringparam1))
    (return true)
    (else
      (return false))))

(fn `BPServerHandleNetExecCommand`
  (params (FromPC :type "PlayerController Object Reference") (CommandName :type Name) (ExecParams :type "BPNetExecParams Structure (by ref)"))
  (returns (ReturnValue :type Boolean))
  (bind _returnvalue (`PrimalAutocastFunctions.PCToSPC` FromPC))
  (if (== CommandName "SheldonChat")
    (set `self.CurrentRequesterPC` _returnvalue)
    (bind _returnvalue_2 (`ShooterPlayerController.GetPlayerCharacterName` _returnvalue))
    (bind _asshooter_player_state (cast `ShooterPlayerState` (`Controller.PlayerState` _returnvalue)))
    (bind _returnvalue_3 (`ShooterPlayerState.GetUniqueNetIdAsString` _asshooter_player_state))
    (`/SheldonAI/Blueprints/BP_SheldonWebSocket.SendPlayerMessage` (`self.SheldonWebSocket`) (`KismetStringLibrary.Concat_StrStr` _returnvalue_3 "|||" (`KismetStringLibrary.Conv_BoolToString` (`PrimalPlayerController.bIsAdmin` _returnvalue)) "|||" _returnvalue_2 "|||" (`.StringParam1` (break `BPNetExecParams` ExecParams))))
    (return true)
    (else
      (return false))))

(fn `OnRep_ExecCommand`
  (bind _returnvalue (`GameplayStatics.GetPlayerController` null))
  (bind (_lefts _rights) (`KismetStringLibrary.Split` (`self.ExecCommand`) "|"))
  (bind _asshooter_player_state (cast `ShooterPlayerState` (`Controller.PlayerState` _returnvalue)))
  (bind _returnvalue_2 (`ShooterPlayerState.GetUniqueNetIdAsString` _asshooter_player_state))
  (if (`KismetStringLibrary.Contains` _returnvalue_2 _lefts)
    (`KismetSystemLibrary.ExecuteConsoleCommand` _returnvalue _rights _returnvalue)))

(fn `OnRep_PinCommand`
  (bind _returnvalue (`GameplayStatics.GetPlayerController` null))
  (bind (_lefts _rights) (`KismetStringLibrary.Split` (`self.PinCommand`) "|"))
  (bind (_lefts_2 _rights_2) (`KismetStringLibrary.Split` _rights "|"))
  (bind _returnvalue_2 (`KismetStringLibrary.Conv_StringToName` _lefts_2))
  (bind (_lefts_3 _rights_3) (`KismetStringLibrary.Split` _rights_2 "|"))
  (bind (_lefts_4 _rights_4) (`KismetStringLibrary.Split` _rights_3 "|"))
  (bind (_lefts_5 _rights_5) (`KismetStringLibrary.Split` _rights_4 "|"))
  (bind (_lefts_6 _rights_6) (`KismetStringLibrary.Split` _rights_5 "|"))
  (bind _asshooter_player_state (cast `ShooterPlayerState` (`Controller.PlayerState` _returnvalue)))
  (bind _returnvalue_3 (`ShooterPlayerState.GetUniqueNetIdAsString` _asshooter_player_state))
  (if (`KismetStringLibrary.Contains` _returnvalue_3 _rights_6)
    (bind _returnvalue_4 (`GameplayStatics.GetCurrentLevelName` null))
    (bind _asshooter_player_controller (cast `ShooterPlayerController` _returnvalue))
    (if (`KismetStringLibrary.Contains` _lefts "add")
      (bind _returnvalue_5 (`KismetStringLibrary.Conv_StringToName` _returnvalue_4))
      (`ShooterPlayerController.NewMinimapMark` _asshooter_player_controller (make `MinimapMark` _lefts_3 _returnvalue_2 (`KismetMathLibrary.MakeVector` (`KismetStringLibrary.Conv_StringToDouble` _lefts_4) (`KismetStringLibrary.Conv_StringToDouble` _lefts_5) (`KismetStringLibrary.Conv_StringToDouble` _lefts_6)) (struct :`G` 1.0 :`B` 1.0 :`A` 1.0) 0 null _returnvalue_5 true))
      (else
        (`ShooterPlayerController.RemoveMinimapMark` _asshooter_player_controller _returnvalue_2 _returnvalue_5)))))

(fn `OnRep_ReplyText`
  (bind _returnvalue (`GameplayStatics.GetPlayerController` null))
  (bind _subtitlewidget (`self.SubtitleWidget`))
  (bind _replytext (`self.ReplyText`))
  (bind _chatwidget (`self.ChatWidget`))
  (bind _asshooter_player_state (cast `ShooterPlayerState` (`Controller.PlayerState` _returnvalue)))
  (bind _returnvalue_2 (`ShooterPlayerState.GetUniqueNetIdAsString` _asshooter_player_state))
  (if (`KismetStringLibrary.Contains` _returnvalue_2 (`self.TargetEos`))
    (set `/SheldonAI/Widgets/WBP_SheldonChat.SheldonMsg` _replytext _chatwidget)
    (`/SheldonAI/Widgets/WBP_SheldonChat.SheldonRenderMessage` _chatwidget)
    (if (not (and (`KismetSystemLibrary.IsValid` _subtitlewidget) (`PrimalUserWidget.IsInViewport` _subtitlewidget)))
      (bind _returnvalue_3 (`|CreateWidget` "/SheldonAI/Widgets/WBP_SheldonSubtitle.WBP_SheldonSubtitle_C" _returnvalue))
      (set `self.SubtitleWidget` _returnvalue_3)
      (`PrimalUserWidget.AddToViewport` _subtitlewidget 100))
    (`/SheldonAI/Widgets/WBP_SheldonSubtitle.ShowSubtitle` _subtitlewidget (`KismetTextLibrary.Conv_StringToText` _replytext))))

(fn `SweepPlayerBuffs`
  (bind _outactors (`GameplayStatics.GetAllActorsOfClass` null "/Script/ShooterGame.ShooterCharacter"))
  (for _array_element _outactors
    (bind _asshooter_character (cast `ShooterCharacter` _array_element))
    (`PrimalBuff.StaticAddBuff` "/SheldonAI/Blueprints/BP_SheldonInputBuff.BP_SheldonInputBuff_C" _asshooter_character null null)))

(fn `UserConstructionScript`)