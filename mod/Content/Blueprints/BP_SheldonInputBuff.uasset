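; Player buff that gives the local player an F8-toggled "Sheldon" chat widget, created on possession and shared with BP_SheldonMapExtension.
; Server net exec commands forward SheldonChat text, with requesting buff and controller, and SheldonTelemetry to the map extension's BP_SheldonWebSocket component.
; SheldonReply commands display responses in the client's widget.
; The client sends telemetry commands without text on possession and when handling client commands.
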(event `Key|F8`
  (params (Key :type "Key Structure"))
  (:`Pressed`
    (if (`self.IsWidgetOpen`)
      (`PrimalUserWidget.RemoveFromViewport` (`self.ChatWidget`))
      (`WidgetBlueprintLibrary.SetInputMode_GameOnly` null)
      (bind _asprimal_player_controller (cast `PrimalPlayerController` (`GameplayStatics.GetPlayerController` null)))
      (set `PrimalPlayerController.bForceShowMouseCursor` false _asprimal_player_controller)
      (set `self.IsWidgetOpen` false)
      (else
        (`PrimalUserWidget.AddToViewport` (`self.ChatWidget`) 0)
        (`WidgetBlueprintLibrary.SetInputMode_UIOnlyEx` null (`self.ChatWidget`))
        (bind _asprimal_player_controller_2 (cast `PrimalPlayerController` (`GameplayStatics.GetPlayerController` null)))
        (set `PrimalPlayerController.bForceShowMouseCursor` true _asprimal_player_controller_2)
        (set `self.IsWidgetOpen` true)))))

(event `self.BPInstigatorLocalPossessed`
  (params (ByController :type "ShooterPlayerController Object Reference"))
  (`self.EnableInput` ByController)
  (bind _returnvalue (`|CreateWidget` "/SheldonAI/Widgets/WBP_SheldonChat.WBP_SheldonChat_C" ByController))
  (bind _output_get (set `self.ChatWidget` _returnvalue))
  (set `/SheldonAI/Widgets/WBP_SheldonChat.MapExtensionRef` self _output_get)
  (`PrimalPlayerController.ClientSendNetExecCommandToServer` ByController self "SheldonTelemetry" (make `BPNetExecParams` :`StringParam1` "__telemetry:client_ready") true)
  (bind _returnvalue_2 (`GameplayStatics.GetActorOfClass` null "/SheldonAI/Blueprints/BP_SheldonMapExtension.BP_SheldonMapExtension_C"))
  (bind _asbp_sheldon_map_extension (cast `/SheldonAI/Blueprints/BP_SheldonMapExtension` _returnvalue_2))
  (set `/SheldonAI/Blueprints/BP_SheldonMapExtension.ChatWidget` (`self.ChatWidget`) _asbp_sheldon_map_extension))

(fn `BPClientHandleNetExecCommand`
  (params (CommandName :type Name) (ExecParams :type "BPNetExecParams Structure (by ref)") (ForPC :type "PlayerController Object Reference"))
  (returns (ReturnValue :type Boolean))
  (bind _returnvalue (`parent.BPClientHandleNetExecCommand` CommandName ExecParams ForPC))
  (bind _asprimal_player_controller (cast `PrimalPlayerController` ForPC))
  (`PrimalPlayerController.ClientSendNetExecCommandToServer` _asprimal_player_controller self "SheldonTelemetry" (make `BPNetExecParams` :`StringParam1` "__telemetry:client_rpc") true)
  (if (== CommandName "SheldonReply")
    (`/SheldonAI/Widgets/WBP_SheldonChat.DisplayResponse` (`self.ChatWidget`) (`.StringParam1` (break `BPNetExecParams` ExecParams)))
    (`PrimalPlayerController.ClientSendNetExecCommandToServer` _asprimal_player_controller self "SheldonTelemetry" (make `BPNetExecParams` :`StringParam1` "__telemetry:displayed") true)
    (return true)
    (else
      (return _returnvalue))))

(fn `BPServerHandleNetExecCommand`
  (params (FromPC :type "PlayerController Object Reference") (CommandName :type Name) (ExecParams :type "BPNetExecParams Structure (by ref)"))
  (returns (ReturnValue :type Boolean))
  (bind (_intparam1 _intparam2 _intparam3 _intarrayparam1 _floatparam1 _floatparam2 _floatparam3 _floatarrayparam1 _objparam1 _objparam2 _objparam3 _stringparam1) (break `BPNetExecParams` ExecParams))
  (bind _returnvalue (`parent.BPServerHandleNetExecCommand` FromPC CommandName ExecParams))
  (if (== CommandName "SheldonChat")
    (bind _returnvalue_2 (`GameplayStatics.GetActorOfClass` null "/SheldonAI/Blueprints/BP_SheldonMapExtension.BP_SheldonMapExtension_C"))
    (bind _asbp_sheldon_web_socket (cast `/SheldonAI/Blueprints/BP_SheldonWebSocket` (`self.GetComponentByClass` _returnvalue_2 "/SheldonAI/Blueprints/BP_SheldonWebSocket.BP_SheldonWebSocket_C")))
    (bind _asprimal_player_controller (cast `PrimalPlayerController` FromPC))
    (`/SheldonAI/Blueprints/BP_SheldonWebSocket.SendFromBuff` _asbp_sheldon_web_socket _stringparam1 self _asprimal_player_controller)
    (elif (== CommandName "SheldonTelemetry")
      (bind _returnvalue_3 (`GameplayStatics.GetActorOfClass` null "/SheldonAI/Blueprints/BP_SheldonMapExtension.BP_SheldonMapExtension_C"))
      (bind _asbp_sheldon_web_socket_2 (cast `/SheldonAI/Blueprints/BP_SheldonWebSocket` (`self.GetComponentByClass` _returnvalue_3 "/SheldonAI/Blueprints/BP_SheldonWebSocket.BP_SheldonWebSocket_C")))
      (`/SheldonAI/Blueprints/BP_SheldonWebSocket.SendPlayerMessage` _asbp_sheldon_web_socket_2 _stringparam1)
      (else
        (return _returnvalue))))
  (return true))

(fn `UserConstructionScript`)